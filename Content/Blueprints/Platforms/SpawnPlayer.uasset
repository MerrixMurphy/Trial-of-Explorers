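; SpawnPlayer is a platform Blueprint that positions the player at level start and themes its cube to match the player's background choice.
; After a tiny BeginPlay delay, it moves the existing player character to the PlayerSpawn component's location and rotation, applying a fixed enlarged scale.
; After a second tiny delay, it reads the character's Backgroundnum to set the Cube material to stone, ice, grass or Purg.
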(event `self.ReceiveBeginPlay`
  (bind (_returnvalue_location _returnvalue_rotation) (`KismetMathLibrary.BreakTransform` (`SceneComponent.K2_GetComponentToWorld` (`self.player_spawn`))))
  (`KismetSystemLibrary.Delay` 0.001)
  (`SceneComponent.K2_SetWorldTransform` (`Actor.RootComponent` (`GameplayStatics.GetPlayerCharacter` 0)) (`KismetMathLibrary.MakeTransform` _returnvalue_location _returnvalue_rotation (7.5 7.5 7.5)) false false)
  (`KismetSystemLibrary.Delay` 0.001)
  (bind _ascharacter (cast `/Game/Blueprints/Actors/Character` (`GameplayStatics.GetPlayerCharacter` 0)))
  (`PrimitiveComponent.SetMaterial` (`self.Cube`) 0 (select `int` (`/Game/Blueprints/Actors/Character.backgroundnum` _ascharacter) :`0` "/Game/Textures/Backgrounds/Cave/Mat/Stone.Stone" :`1` "/Game/Textures/Backgrounds/Mountains/Mat/ice.ice" :`2` "/Game/Textures/Backgrounds/Forest/Mat/Grass1.Grass1" :`3` "/Game/Textures/Backgrounds/Purgatory/Mat/Purg.Purg" :!type "MaterialInterface Object Reference")))

(fn `UserConstructionScript`)