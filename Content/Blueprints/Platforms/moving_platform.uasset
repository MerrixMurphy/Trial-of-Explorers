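; A moving platform that slides its cube back and forth along a timeline path and skins it to match the current background.
; Shortly after BeginPlay, it picks a stone, ice, grass or purgatory material from the player Character's Backgroundnum.
; The Move timeline sets the cube's swept relative location after a random start delay.
; A Delay on the timeline's Update and the Looped flag alternate between reversing and replaying with a new random delay.
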(event `self.ReceiveBeginPlay`
  (`KismetSystemLibrary.Delay` 0.1)
  (bind _ascharacter (cast `/Game/Blueprints/Actors/Character` (`GameplayStatics.GetPlayerCharacter` 0)))
  (`PrimitiveComponent.SetMaterial` (`self.Cube1`) 0 (select `int` (`/Game/Blueprints/Actors/Character.backgroundnum` _ascharacter) :`0` "/Game/Textures/Backgrounds/Cave/Mat/Stone.Stone" :`1` "/Game/Textures/Backgrounds/Mountains/Mat/ice.ice" :`2` "/Game/Textures/Backgrounds/Forest/Mat/Grass1.Grass1" :`3` "/Game/Textures/Backgrounds/Purgatory/Mat/Purg.Purg" :!type "MaterialInterface Object Reference"))
  (`KismetSystemLibrary.Delay` (`KismetMathLibrary.RandomFloatInRange` 0.0 2.0) :!label _label)
  (bind (_direction _newtrack_0) (`Timeline|move` :!label _label_2)
    (:`Update`
      (`SceneComponent.K2_SetRelativeLocation` (`self.Cube1`) _newtrack_0 true false)
      (`KismetSystemLibrary.Delay` 3.0)
      (if (`self.looped`)
        (set `self.looped` false)
        (goto _label_2 :!via `Reverse`)
        (else
          (set `self.looped` true)
          (goto _label))))))

(fn `UserConstructionScript`)