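; SpawnFinish is the finish-line platform that ends a level with a victory when the player reaches it.
; Shortly after BeginPlay it sets the cube's material from the player Character's Backgroundnum, choosing stone, ice, grass or purgatory themes.
; When a Character overlaps the box, it plays a victory sound, scores the run from time alive, pauses the game and shows Background and Victory widgets.
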(event `self.ReceiveBeginPlay`
  (`KismetSystemLibrary.Delay` 0.1)
  (bind _ascharacter (cast `/Game/Blueprints/Actors/Character` (`GameplayStatics.GetPlayerCharacter` 0)))
  (`PrimitiveComponent.SetMaterial` (`self.Cube`) 0 (select `int` (`/Game/Blueprints/Actors/Character.backgroundnum` _ascharacter) :`0` "/Game/Textures/Backgrounds/Cave/Mat/Stone.Stone" :`1` "/Game/Textures/Backgrounds/Mountains/Mat/ice.ice" :`2` "/Game/Textures/Backgrounds/Forest/Mat/Grass1.Grass1" :`3` "/Game/Textures/Backgrounds/Purgatory/Mat/Purg.Purg" :!type "MaterialInterface Object Reference")))

(event `self.Box.OnComponentBeginOverlap`
  (params (OverlappedComponent :type "PrimitiveComponent Object Reference") (OtherActor :type "Actor Object Reference") (OtherComp :type "PrimitiveComponent Object Reference") (OtherBodyIndex :type Integer) (bFromSweep :type Boolean) (SweepResult :type "HitResult Structure (by ref)"))
  (cast `/Game/Blueprints/Actors/Character` OtherActor)
  (`GameplayStatics.PlaySound2D` "/Game/Sounds/victory.victory" 1.0 1.0 0.0 null null)
  (bind _returnvalue (`|CreateWidget` "/Game/Blueprints/UI/background.background_C"))
  (`UserWidget.AddToViewport` _returnvalue 0)
  (bind _ascharacter (cast `/Game/Blueprints/Actors/Character` (`GameplayStatics.GetPlayerCharacter` 0)))
  (set `/Game/Blueprints/Actors/Character.VictoryScore` (- 1200 (`/Game/Blueprints/Actors/Character.TimeAlive` _ascharacter)) _ascharacter)
  (`GameplayStatics.SetGamePaused` true)
  (bind _returnvalue_2 (`|CreateWidget` "/Game/Blueprints/UI/Victory.Victory_C"))
  (`UserWidget.AddToViewport` _returnvalue_2 0))

(fn `UserConstructionScript`)