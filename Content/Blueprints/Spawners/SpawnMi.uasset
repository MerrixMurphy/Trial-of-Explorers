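; SpawnMi is a spawner that populates its Box volume with monsters, an optional boss and coins on BeginPlay.
; It spawns random counts of monsters and coins within configurable ranges, plus one boss if the Boss class is set.
; Each spawn helper picks a random point in the box, with rotations of only 0–1 degree per axis.
; Monster spawns may fail on collision, while boss and coins always spawn.
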(event `self.ReceiveBeginPlay`
  (`|ExecutionSequence`
    (:`then_1`
      (for _ (range 1 (+ (`KismetMathLibrary.RandomIntegerInRange` (`self.min_monsters`) (`self.max_monsters`)) 1))
        (`self.SpawnMon`)))
    (:`then_2`
      (if (`self.Boss`)
        (`self.SpawnBoss`)))
    (:`then_3`
      (for _ (range 1 (+ (`KismetMathLibrary.RandomIntegerInRange` (`self.min_coins`) (`self.max_coins`)) 1))
        (`self.SpawnCoin`)))))

(fn `SpawnBoss`
  (bind _returnvalue (`KismetMathLibrary.RandomFloat`))
  (bind (_origin _boxextent) (`KismetSystemLibrary.GetComponentBounds` (`self.Box`)))
  (`|SpawnActorFromClass` "/Game/Blueprints/Actors/Boss.Boss_C" (`KismetMathLibrary.MakeTransform` (`KismetMathLibrary.RandomPointInBoundingBox` _origin _boxextent) (`KismetMathLibrary.MakeRotator` _returnvalue _returnvalue _returnvalue)) "AdjustIfPossibleButAlwaysSpawn" "OverrideRootScale" null null))

(fn `SpawnCoin`
  (bind _returnvalue (`KismetMathLibrary.RandomFloat`))
  (bind (_origin _boxextent) (`KismetSystemLibrary.GetComponentBounds` (`self.Box`)))
  (`|SpawnActorFromClass` "/Game/Blueprints/Actors/Coin.Coin_C" (`KismetMathLibrary.MakeTransform` (`KismetMathLibrary.RandomPointInBoundingBox` _origin _boxextent) (`KismetMathLibrary.MakeRotator` _returnvalue _returnvalue _returnvalue)) "AdjustIfPossibleButAlwaysSpawn" "OverrideRootScale" null null))

(fn `SpawnMon`
  (bind _returnvalue (`KismetMathLibrary.RandomFloat`))
  (bind (_origin _boxextent) (`KismetSystemLibrary.GetComponentBounds` (`self.Box`)))
  (`|SpawnActorFromClass` "/Game/Blueprints/Actors/Monsters.Monsters_C" (`KismetMathLibrary.MakeTransform` (`KismetMathLibrary.RandomPointInBoundingBox` _origin _boxextent) (`KismetMathLibrary.MakeRotator` _returnvalue _returnvalue _returnvalue)) "AdjustIfPossibleButDontSpawnIfColliding" "OverrideRootScale" null null))

(fn `UserConstructionScript`)