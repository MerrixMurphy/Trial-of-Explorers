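; Floor actor that matches its look to the background chosen on the player character.
; Shortly after BeginPlay it reads the character's Backgroundnum and sets its static mesh to a stone, ice, grass or purg material.
; Every Tick it re-casts the player character and shows the floor only while CameraActive is true, hiding it otherwise.
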(event `self.ReceiveBeginPlay`
  (`KismetSystemLibrary.Delay` 0.1)
  (bind _ascharacter (cast `/Game/Blueprints/Actors/Character` (`GameplayStatics.GetPlayerCharacter` 0)))
  (`PrimitiveComponent.SetMaterial` (`self.StaticMeshComponent`) 0 (select `int` (`/Game/Blueprints/Actors/Character.backgroundnum` _ascharacter) :`0` "/Game/Textures/Backgrounds/Cave/Mat/Stone.Stone" :`1` "/Game/Textures/Backgrounds/Mountains/Mat/ice.ice" :`2` "/Game/Textures/Backgrounds/Forest/Mat/Grass.Grass" :`3` "/Game/Textures/Backgrounds/Purgatory/Mat/Purg.Purg" :!type "MaterialInterface Object Reference")))

(event `self.ReceiveTick`
  (params (DeltaSeconds :type "Float (single-precision)"))
  (bind _ascharacter (cast `/Game/Blueprints/Actors/Character` (`GameplayStatics.GetPlayerCharacter` 0)))
  (if (`/Game/Blueprints/Actors/Character.cameraActive` _ascharacter)
    (`self.SetActorHiddenInGame` false)
    (else
      (`self.SetActorHiddenInGame` true))))

(fn `UserConstructionScript`)