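; Boss enemy character with flipbook sprites that wanders the level and ends the game when a character overlaps its box.
; It roams by looping AI MoveTo to random reachable points, retrying on failure as well.
; Each tick it picks a jumping, falling, moving or idle flipbook from velocity, indexed by a random variant that currently always resolves to Wilderman.
; On overlap it hides that character, shows end and game-over widgets, and pauses.
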(event `self.ReceiveTick`
  (params (DeltaSeconds :type "Float (single-precision)"))
  ;[1 1 1] On Tick
  (`self.MoveAnimation`))

(event `self.ReceiveBeginPlay`
  ;[1 1 1] On start
  (`self.setNum`)
  (`self.roam`))

(event `MoveAnimation`
  (bind (_returnvalue_x _returnvalue_y _returnvalue_z) (`KismetMathLibrary.BreakVector` (`self.GetVelocity`)))
  (bind _sprite (`self.Sprite`))
  ;[1 1 1] Start Animation/Check Falling
  (if (`NavMovementComponent.IsFalling` (`self.CharacterMovement`))
    (`PaperFlipbookComponent.SetFlipbook` _sprite (select `bool` (> _returnvalue_z 0.0) :`false` (select `int` (stale `setNum` _output_get) :`0` "/Game/Flipbooks/Characters/Wildman/Falling_Wilderman.Falling_Wilderman" :`1` null :!type "PaperFlipbook Object Reference") :`true` (select `int` (stale `setNum` _output_get) :`0` "/Game/Flipbooks/Characters/Wildman/Jumping_Wilderman.Jumping_Wilderman" :`1` null :!type "PaperFlipbook Object Reference")))
    (else
      (`PaperFlipbookComponent.SetFlipbook` _sprite (select `bool` (> (`KismetMathLibrary.VSize` (`MovementComponent.Velocity` (`self.CharacterMovement`))) 0.0) :`false` (select `int` (stale `setNum` _output_get) :`0` "/Game/Flipbooks/Characters/Wildman/idle_Wilderman.idle_Wilderman" :`1` null :!type "PaperFlipbook Object Reference") :`true` (select `int` (stale `setNum` _output_get) :`0` "/Game/Flipbooks/Characters/Wildman/Moving_Wilderman.Moving_Wilderman" :`1` null :!type "PaperFlipbook Object Reference"))))))

(event `roam`
  ;[1 1 1] Movement
  (`|AIMoveTo` self (`NavigationSystemV1.K2_GetRandomReachablePointInRadius` (`self.K2_GetActorLocation`) 1000.0 null null) null
    (:`OnSuccess`
      _)
    (:`OnFail`
      _))
  (`self.roam`))

(event `setNum`
  ;[1 1 1] Ran Gen
  (bind _output_get (set `self.Ran` (`KismetMathLibrary.RandomIntegerInRange` 0))))

(event `self.Box.OnComponentBeginOverlap`
  (params (OverlappedComponent :type "PrimitiveComponent Object Reference") (OtherActor :type "Actor Object Reference") (OtherComp :type "PrimitiveComponent Object Reference") (OtherBodyIndex :type Integer) (bFromSweep :type Boolean) (SweepResult :type "HitResult Structure (by ref)"))
  (bind _ascharacter (cast `/Game/Blueprints/Character` OtherActor))
  (`self.SetActorHiddenInGame` _ascharacter true)
  (bind _returnvalue (`|CreateWidget` "/Game/Blueprints/EndUI.EndUI_C"))
  (`UserWidget.AddToViewport` _returnvalue 0)
  (bind _returnvalue_2 (`|CreateWidget` "/Game/Blueprints/GameOver.GameOver_C"))
  (`UserWidget.AddToViewport` _returnvalue_2 0)
  (`GameplayStatics.SetGamePaused` true))

(fn `UserConstructionScript`)