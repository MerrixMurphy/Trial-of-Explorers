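; Minion creates a grid-indexed set of streaming level instances when play begins.
; Nested loops over NumX and NumY call CreateInstance on a looked-up streaming level, naming each copy from its indices joined by an X.
; The level lookup name is None, and the graph sets no transform, loading or visibility on the created instances.
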(event `self.ReceiveBeginPlay`
  (for _index (range (`self.NumX`))
    (set `self.LoopX` _index)
    (for _index_2 (range (`self.NumY`))
      (set `self.LoopY` _index_2)
      (`LevelStreaming.CreateInstance` (`GameplayStatics.GetStreamingLevel` "None") (`KismetStringLibrary.Concat_StrStr` (`KismetStringLibrary.Conv_IntToString` (`self.LoopX`)) "X" (`KismetStringLibrary.Conv_IntToString` (`self.LoopY`)))))))

(fn `UserConstructionScript`)