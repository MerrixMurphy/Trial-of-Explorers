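; Level spawner that randomly fills a box volume with platforms, monsters, a boss and coins on BeginPlay.
; Spawns random counts within min/max ranges, picking each platform from seven types and enlarging it.
; The boss and coins spawn only when Boss is set.
; Each actor gets a random point in the box; monsters and coins are skipped if still colliding, while the boss always spawns.
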(event `self.ReceiveBeginPlay`
  (for _ (range 1 (+ (`KismetMathLibrary.RandomIntegerInRange` (`self.min_platforms`) (`self.max_platforms`)) 1))
    (`self.SpawnPlat`))
  (for _ (range 1 (+ (`KismetMathLibrary.RandomIntegerInRange` (`self.min_monsters`) (`self.max_monsters`)) 1))
    (`self.SpawnMon`))
  (if (`self.Boss`)
    (`self.SpawnBoss`)
    (for _ (range 1 (+ (`KismetMathLibrary.RandomIntegerInRange` (`self.min_coins`) (`self.max_coins`)) 1))
      (`self.SpawnCoin`))))

(fn `SpawnBoss`
  (bind _returnvalue (`KismetMathLibrary.RandomFloat`))
  (bind (_origin _boxextent) (`KismetSystemLibrary.GetComponentBounds` (`self.Box`)))
  (`|SpawnActorFromClass` "/Game/Blueprints/Boss.Boss_C" (`KismetMathLibrary.MakeTransform` (`KismetMathLibrary.RandomPointInBoundingBox` _origin _boxextent) (`KismetMathLibrary.MakeRotator` _returnvalue _returnvalue _returnvalue)) "AdjustIfPossibleButAlwaysSpawn" "OverrideRootScale" null null))

(fn `SpawnCoin`
  (bind _returnvalue (`KismetMathLibrary.RandomFloat`))
  (bind (_origin _boxextent) (`KismetSystemLibrary.GetComponentBounds` (`self.Box`)))
  (`|SpawnActorFromClass` "/Game/Blueprints/Coin.Coin_C" (`KismetMathLibrary.MakeTransform` (`KismetMathLibrary.RandomPointInBoundingBox` _origin _boxextent) (`KismetMathLibrary.MakeRotator` _returnvalue _returnvalue _returnvalue)) "AdjustIfPossibleButDontSpawnIfColliding" "OverrideRootScale" null null))

(fn `SpawnMon`
  (bind _returnvalue (`KismetMathLibrary.RandomFloat`))
  (bind (_origin _boxextent) (`KismetSystemLibrary.GetComponentBounds` (`self.Box`)))
  (`|SpawnActorFromClass` "/Game/Blueprints/Monsters.Monsters_C" (`KismetMathLibrary.MakeTransform` (`KismetMathLibrary.RandomPointInBoundingBox` _origin _boxextent) (`KismetMathLibrary.MakeRotator` _returnvalue _returnvalue _returnvalue)) "AdjustIfPossibleButDontSpawnIfColliding" "OverrideRootScale" null null))

(fn `SpawnPlat`
  (bind _returnvalue (`KismetMathLibrary.RandomFloat`))
  (bind (_origin _boxextent) (`KismetSystemLibrary.GetComponentBounds` (`self.Box`)))
  (`|SpawnActorFromClass` (select `int` (`KismetMathLibrary.RandomIntegerInRange` 0 6) :`0` "/Game/Blueprints/flat_platform.flat_platform_C" :`1` "/Game/Blueprints/tri_platform.tri_platform_C" :`2` "/Game/Blueprints/gap_platform.gap_platform_C" :`3` "/Game/Blueprints/spike_platform.spike_platform_C" :`4` "/Game/Blueprints/twin_pillars_platform.twin_pillars_platform_C" :`5` "/Game/Blueprints/wall_platform.wall_platform_C" :`6` "/Game/Blueprints/moving_platform.moving_platform_C" :!type "Actor Class Reference") (`KismetMathLibrary.MakeTransform` (`KismetMathLibrary.RandomPointInBoundingBox` _origin _boxextent) (`KismetMathLibrary.MakeRotator` _returnvalue _returnvalue _returnvalue) (7.5 7.5 7.5)) (`self.Collision Handling Override`) "OverrideRootScale" null null))

(fn `UserConstructionScript`)