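; Spike platform hazard that ends the game for characters touching its box trigger and destroys monsters that hit it.
; On overlap, a sequence casts the other actor to Character, hides it, adds the EndUI and GameOver widgets to the viewport, and pauses the game.
; A second branch casts to Monsters, destroys that actor, and forces garbage collection.
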(event `self.Box.OnComponentBeginOverlap`
  (params (OverlappedComponent :type "PrimitiveComponent Object Reference") (OtherActor :type "Actor Object Reference") (OtherComp :type "PrimitiveComponent Object Reference") (OtherBodyIndex :type Integer) (bFromSweep :type Boolean) (SweepResult :type "HitResult Structure (by ref)"))
  (`|ExecutionSequence`
    (:`then_0`
      (bind _ascharacter (cast `/Game/Blueprints/Character` OtherActor))
      (`self.SetActorHiddenInGame` _ascharacter true)
      (bind _returnvalue (`|CreateWidget` "/Game/Blueprints/EndUI.EndUI_C"))
      (`UserWidget.AddToViewport` _returnvalue 0)
      (bind _returnvalue_2 (`|CreateWidget` "/Game/Blueprints/GameOver.GameOver_C"))
      (`UserWidget.AddToViewport` _returnvalue_2 0)
      (`GameplayStatics.SetGamePaused` true))
    (:`then_1`
      (bind _asmonsters (cast `/Game/Blueprints/Monsters` OtherActor))
      (`self.K2_DestroyActor` _asmonsters)
      (`KismetSystemLibrary.CollectGarbage`))))

(fn `UserConstructionScript`)