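; Paper2D boss character that wanders the level and ends the game when a Character overlaps its box.
; On BeginPlay it randomly picks one of four looks (barrel, dino, trash, tooth), then endlessly chains AI moves to random reachable nearby points.
; Each tick selects that look's idle, run or jump flipbook from movement state.
; Overlap hides the Character, plays a defeat sound, adds the game-over and score widgets, and pauses the game.
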(event `self.ReceiveTick`
  (params (DeltaSeconds :type "Float (single-precision)"))
  ;[1 1 1] On Tick
  (`self.MoveAnimation`))

(event `self.ReceiveBeginPlay`
  ;[1 1 1] On start
  (`self.setNum`)
  (`self.roam`))

(event `MoveAnimation`
  (bind (_returnvalue_x _returnvalue_y _returnvalue_z) (`KismetMathLibrary.BreakVector` (`self.GetVelocity`)))
  (bind _sprite (`self.Sprite`))
  ;[1 1 1] Start Animation/Check Falling
  (if (`NavMovementComponent.IsFalling` (`self.CharacterMovement`))
    (`PaperFlipbookComponent.SetFlipbook` _sprite (select `bool` (> _returnvalue_z 0.0) :`false` (select `int` (stale `setNum` _output_get) :`0` "/Game/Flipbooks/Bosses/Barrel_Knight/Run/barrel_boss_run.barrel_boss_run" :`1` "/Game/Flipbooks/Bosses/Trash_Monster/Run/dino_run.dino_run" :`2` "/Game/Flipbooks/Bosses/Trash_Monster/Run/trash_run.trash_run" :`3` "/Game/Flipbooks/Bosses/tooth_walker/Run/tooth_run.tooth_run" :!type "PaperFlipbook Object Reference") :`true` (select `int` (stale `setNum` _output_get) :`0` "/Game/Flipbooks/Bosses/Barrel_Knight/Jump/barrel_boss_jump.barrel_boss_jump" :`1` "/Game/Flipbooks/Bosses/Trash_Monster/Jump/dino_jump.dino_jump" :`2` "/Game/Flipbooks/Bosses/Trash_Monster/Jump/trash_jump.trash_jump" :`3` "/Game/Flipbooks/Bosses/tooth_walker/Jump/tooth_jump.tooth_jump" :!type "PaperFlipbook Object Reference")))
    (else
      (`PaperFlipbookComponent.SetFlipbook` _sprite (select `bool` (> (`KismetMathLibrary.VSize` (`MovementComponent.Velocity` (`self.CharacterMovement`))) 0.0) :`false` (select `int` (stale `setNum` _output_get) :`0` "/Game/Flipbooks/Bosses/Barrel_Knight/Idle/barrel_boss_idle.barrel_boss_idle" :`1` "/Game/Flipbooks/Bosses/Trash_Monster/Idle/dino_idle.dino_idle" :`2` "/Game/Flipbooks/Bosses/Trash_Monster/Idle/trash_idle.trash_idle" :`3` "/Game/Flipbooks/Bosses/tooth_walker/Idle/tooth_idle.tooth_idle" :!type "PaperFlipbook Object Reference") :`true` (select `int` (stale `setNum` _output_get) :`0` "/Game/Flipbooks/Bosses/Barrel_Knight/Run/barrel_boss_run.barrel_boss_run" :`1` "/Game/Flipbooks/Bosses/Trash_Monster/Run/dino_run.dino_run" :`2` "/Game/Flipbooks/Bosses/Trash_Monster/Run/trash_run.trash_run" :`3` "/Game/Flipbooks/Bosses/tooth_walker/Run/tooth_run.tooth_run" :!type "PaperFlipbook Object Reference"))))))

(event `roam`
  ;[1 1 1] Movement
  (`|AIMoveTo` self (`NavigationSystemV1.K2_GetRandomReachablePointInRadius` (`self.K2_GetActorLocation`) 1000.0 null null) null
    (:`OnSuccess`
      _)
    (:`OnFail`
      _))
  (`self.roam`))

(event `setNum`
  ;[1 1 1] Ran Gen
  (bind _output_get (set `self.Ran` (`KismetMathLibrary.RandomIntegerInRange` 0 3))))

(event `self.Box.OnComponentBeginOverlap`
  (params (OverlappedComponent :type "PrimitiveComponent Object Reference") (OtherActor :type "Actor Object Reference") (OtherComp :type "PrimitiveComponent Object Reference") (OtherBodyIndex :type Integer) (bFromSweep :type Boolean) (SweepResult :type "HitResult Structure (by ref)"))
  (bind _ascharacter (cast `/Game/Blueprints/Actors/Character` OtherActor))
  (`self.SetActorHiddenInGame` _ascharacter true)
  (`GameplayStatics.PlaySound2D` "/Game/Sounds/Fallen_in_Battle_Cue.Fallen_in_Battle_Cue" 1.0 1.0 0.0 null null)
  (bind _returnvalue (`|CreateWidget` "/Game/Blueprints/UI/background.background_C"))
  (`UserWidget.AddToViewport` _returnvalue 0)
  (bind _returnvalue_2 (`|CreateWidget` "/Game/Blueprints/UI/GameOver.GameOver_C"))
  (`UserWidget.AddToViewport` _returnvalue_2 0)
  (bind _returnvalue_3 (`|CreateWidget` "/Game/Blueprints/UI/EndUI.EndUI_C"))
  (`UserWidget.AddToViewport` _returnvalue_3 0)
  (bind _returnvalue_4 (`|CreateWidget` "/Game/Blueprints/UI/HighScore.HighScore_C"))
  (`UserWidget.AddToViewport` _returnvalue_4 0)
  (`GameplayStatics.SetGamePaused` true))

(fn `UserConstructionScript`)